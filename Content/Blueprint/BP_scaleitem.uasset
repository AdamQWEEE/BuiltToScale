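; BP_scaleitem is an actor that grows as the third-person player character gets closer.
; Each Tick it looks up BP_ThirdPersonCharacter with GetActorOfClass and measures the distance between the two.
; Within 1500 units it sets a uniform scale that rises linearly from about 1 at the edge to 3 at zero distance.
; Outside that range the scale is left unchanged; a distance debug print is disconnected.
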(event EventBeginPlay)

(event Collision|EventActorBeginOverlap
  (params (OtherActor :type Actor%20Object%20Reference)))

(event EventTick
  (params (DeltaSeconds :type Float%20%28single-precision%29))
  (bind _returnvalue (Actor|GetActorOfClass "/Game/ThirdPerson/Blueprints/BP_ThirdPersonCharacter.BP_ThirdPersonCharacter_C"))
  (if (< (Math|Vector|VectorLength (- (Transformation|GetActorLocation _returnvalue) (Transformation|GetActorLocation))) 1.5e+03)
    (Transformation|SetActorScale3D (* (/ (- 3e+03 (* (Math|Vector|VectorLength (- (Transformation|GetActorLocation _returnvalue) (Transformation|GetActorLocation))) 1.3333)) 1e+03) "1.000000,1.000000,1.000000"))))

(fn ConstructionScript)